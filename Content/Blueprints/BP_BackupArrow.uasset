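; BP_BackupArrow is an arrow projectile whose launch speed scales with bow charge.
; The construction script loops over every BP_Bow, setting and printing InitialSpeed from ChargeAmount times SpeedMultiplier, so the last bow wins.
; BeginPlay sets move-ignores for itself and its collision owner; a hit deactivates Collision, and projectile stop halts rotation and disables physics simulation.
; Deprecated, unconnected logic once aimed the arrow at the player's camera raycast endpoint.
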(event OnComponentHit(Collision)
  (params (HitComponent :type Primitive%20Component%20Object%20Reference) (OtherActor :type Actor%20Object%20Reference) (OtherComp :type Primitive%20Component%20Object%20Reference) (NormalImpulse :type Vector :default "0, 0, 0") (Hit :type Hit%20Result%20Structure%20%28by%20ref%29))
  (Components|Activation|Deactivate (Variables|Default|GetCollision)))

(event OnProjectileStop(ProjectileMovement)
  (params (ImpactResult :type Hit%20Result%20Structure%20%28by%20ref%29))
  (Variables|/Script/Engine.RotatingMovementComponent|SetRotationRate (Variables|Default|GetRotatingMovement) "0, 0, 0")
  (Physics|SetSimulatePhysics (Variables|Default|GetCollision) false))

(event EventBeginPlay
  (bind _collision (Variables|Default|GetCollision))
  (Collision|IgnoreActorwhenMoving (Variables|Default|GetCollision) (Components|GetOwner (Variables|Default|GetCollision)) true)
  (Collision|IgnoreActorwhenMoving (Variables|Default|GetCollision) self true)
  (Class|PrimitiveComponent|IgnoreComponentwhenMoving _collision _collision true))

(fn ConstructionScript
  (bind _outactors (Actor|GetAllActorsOfClass "/Game/Blueprints/BP_Bow.BP_Bow_C"))
  (for _array_element _outactors
    (bind _output_get (Variables|Default|SetSpeed (* (Variables|/Game/Blueprints/BP_Bow.BP_Bow_C|GetChargeAmount _array_element) (Variables|Default|GetSpeed%20Multiplier))))
    (Development|PrintString (Utilities|String|ToString(Float) _output_get))
    (Variables|/Script/Engine.ProjectileMovementComponent|SetInitialSpeed (Variables|Default|GetProjectileMovement) _output_get)))