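; Monster plant enemy that either stands still as a fireball turret or chases and melees the player, chosen by IsStatic.
; Static plants loop an attack that aims at the player and spawns BP_Fireball; IsHomingProjectile skips the spawn and loop.
; Tick issues AIMoveTo at the player controller, and capsule hits on the player trigger delayed damage for mobile plants.
; One BP_NewArrow hit kills it, destroying both after the hit animation.
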(event OnComponentHit(CapsuleComponent)
  (params (HitComponent :type Primitive%20Component%20Object%20Reference) (OtherActor :type Actor%20Object%20Reference) (OtherComp :type Primitive%20Component%20Object%20Reference) (NormalImpulse :type Vector :default "0, 0, 0") (Hit :type Hit%20Result%20Structure%20%28by%20ref%29))
  (bind _mesh (Variables|Character|GetMesh))
  (bind _asbp_new_arrow (Utilities|Casting|CastToBP_NewArrow OtherActor)
    (:then
      (Variables|Default|SetisDead? true)
      (Collision|SetCollisionEnabled (Variables|Collision|GetCapsuleComponent) "NoCollision")
      (Components|Animation|PlayAnimation _mesh "/Game/Assets/PlantMonster/Animations/GotHit.GotHit" false)
      (Components|Timeline|SetPlayRate _mesh 1.5)
      (Development|PrintString "Hit")
      (Utilities|FlowControl|Delay 1.2)
      (Actor|DestroyActor)
      (Actor|DestroyActor _asbp_new_arrow))
    (:CastFailed
      (if (not (Variables|Default|GetisStatic))
        (if (not (Variables|Default|GetisAttacking?))
          (Utilities|Casting|CastToPlayerCharacter OtherActor)
          (Components|Animation|PlayAnimation (Variables|Character|GetMesh) "/Game/Assets/PlantMonster/Animations/Attack01.Attack01" false)
          (Variables|Default|SetisAttacking? true)
          (Utilities|FlowControl|Delay 0.7)
          (if (not (Variables|Default|GetisDead?))
            (Game|Damage|ApplyDamage (Game|GetPlayerCharacter 0) (Variables|Default|GetattackPower) 0 0)
            (Utilities|FlowControl|Delay 1.2)
            (Variables|Default|SetisAttacking? false)
            (Components|Animation|PlayAnimation (Variables|Character|GetMesh) "/Game/Assets/PlantMonster/Animations/AttackIdle.AttackIdle" true)
            (Development|PrintString "character")))))))

(event EventTick
  (params (DeltaSeconds :type Float%20%28single-precision%29))
  (if (Variables|Default|GetisDead?)
    (Components|Movement|StopMovementImmediately (Variables|Character|GetCharacterMovement))
    (else
      (AI|AIMoveTo self "0, 0, 0" (Game|GetPlayerController 0) (Variables|Default|GetAttackDistance) false
        (:then
          (if (<= (- (Math|Vector|Distance(Vector) (Transformation|GetActorLocation) (Transformation|GetActorLocation (Game|GetPlayerCharacter 0))) 1e+02) (Variables|Default|GetAttackDistance))
            _))))))

(event EventBeginPlay
  (bind _spawnprojectile (Variables|Default|GetSpawnProjectile))
  (if (Variables|Default|GetisStatic)
    (Variables|/Script/Engine.CharacterMovementComponent|SetMaxWalkSpeed (Variables|Character|GetCharacterMovement) 0.0)
    (Components|Animation|PlayAnimation (Variables|Character|GetMesh) "/Game/Assets/PlantMonster/Animations/Attack01.Attack01" false :!label _label)
    (Transformation|SetWorldRotation _spawnprojectile (Math|Rotator|FindLookatRotation (Transformation|GetWorldLocation _spawnprojectile) (Transformation|GetActorLocation (Game|GetPlayerCharacter 0))) false false)
    (if (not (Variables|Default|GetisHomingProjectile?))
      (Utilities|FlowControl|Delay 0.5)
      (Game|SpawnActorfromClass "/Game/Blueprints/BP_Fireball.BP_Fireball_C" (Transformation|GetWorldTransform (Variables|Default|GetSpawnProjectile)) "Undefined" 0 0)
      (Utilities|FlowControl|Delay 1.5)
      (if (not (Variables|Default|GetisDead?))
        (goto _label)))))

(fn ConstructionScript)