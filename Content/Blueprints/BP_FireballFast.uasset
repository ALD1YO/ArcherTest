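; BP_FireballFast is a homing fireball projectile that hunts the player and can be shot down by arrows.
; On BeginPlay it sets the player character's capsule as the ProjectileMovement homing target and starts its lifespan timer.
; A sphere overlap with the player applies fixed damage and destroys the fireball.
; A hit against a BP_NewArrow destroys both the arrow and the fireball.
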(event OnComponentBeginOverlap(Sphere1)
  (params (OverlappedComponent :type Primitive%20Component%20Object%20Reference) (OtherActor :type Actor%20Object%20Reference) (OtherComp :type Primitive%20Component%20Object%20Reference) (OtherBodyIndex :type Integer) (bFromSweep :type Boolean) (SweepResult :type Hit%20Result%20Structure%20%28by%20ref%29))
  (bind _asplayer_character (Utilities|Casting|CastToPlayerCharacter OtherActor))
  (Game|Damage|ApplyDamage _asplayer_character 2e+01 0 0)
  (Actor|DestroyActor))

(event EventBeginPlay
  (Variables|/Script/Engine.ProjectileMovementComponent|SetHomingTargetComponent (Variables|Default|GetProjectileMovement) (Actor|GetComponentbyClass (Game|GetPlayerCharacter 0) "/Script/Engine.CapsuleComponent"))
  (Actor|SetLifeSpan self (Variables|Default|GetlifeSpan)))

(event Collision|EventHit
  (params (MyComp :type Primitive%20Component%20Object%20Reference) (Other :type Actor%20Object%20Reference) (OtherComp :type Primitive%20Component%20Object%20Reference) (bSelfMoved :type Boolean) (HitLocation :type Vector :default "0, 0, 0") (HitNormal :type Vector :default "0, 0, 0") (NormalImpulse :type Vector :default "0, 0, 0") (Hit :type Hit%20Result%20Structure%20%28by%20ref%29))
  (bind _asbp_new_arrow (Utilities|Casting|CastToBP_NewArrow Other))
  (Actor|DestroyActor _asbp_new_arrow)
  (Actor|DestroyActor))

(fn ConstructionScript)