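; Archery target actor with five colored hit components that award more points from white through black, blue and red to yellow.
; Component hit events pass a point value to AddToScore, which counts only BP_NewArrow hits and adds to the Score on the cached MyGameMode.
; The construction script sets InterpToMovement's two relative control points and duration from variables to move the target.
; Two timeline-based lerp movement snippets are unconnected and never run.
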(event OnComponentHit(Target_Black)
  (params (HitComponent :type Primitive%20Component%20Object%20Reference) (OtherActor :type Actor%20Object%20Reference) (OtherComp :type Primitive%20Component%20Object%20Reference) (NormalImpulse :type Vector :default "0, 0, 0") (Hit :type Hit%20Result%20Structure%20%28by%20ref%29))
  (CallFunction|AddtoScore OtherActor 2))

(event OnComponentHit(Target_White)
  (params (HitComponent :type Primitive%20Component%20Object%20Reference) (OtherActor :type Actor%20Object%20Reference) (OtherComp :type Primitive%20Component%20Object%20Reference) (NormalImpulse :type Vector :default "0, 0, 0") (Hit :type Hit%20Result%20Structure%20%28by%20ref%29))
  (CallFunction|AddtoScore OtherActor 1))

(event OnComponentHit(Target_Blue)
  (params (HitComponent :type Primitive%20Component%20Object%20Reference) (OtherActor :type Actor%20Object%20Reference) (OtherComp :type Primitive%20Component%20Object%20Reference) (NormalImpulse :type Vector :default "0, 0, 0") (Hit :type Hit%20Result%20Structure%20%28by%20ref%29))
  (CallFunction|AddtoScore OtherActor 3))

(event OnComponentHit(Target_Red)
  (params (HitComponent :type Primitive%20Component%20Object%20Reference) (OtherActor :type Actor%20Object%20Reference) (OtherComp :type Primitive%20Component%20Object%20Reference) (NormalImpulse :type Vector :default "0, 0, 0") (Hit :type Hit%20Result%20Structure%20%28by%20ref%29))
  (CallFunction|AddtoScore OtherActor 4))

(event OnComponentHit(Target_Yellow)
  (params (HitComponent :type Primitive%20Component%20Object%20Reference) (OtherActor :type Actor%20Object%20Reference) (OtherComp :type Primitive%20Component%20Object%20Reference) (NormalImpulse :type Vector :default "0, 0, 0") (Hit :type Hit%20Result%20Structure%20%28by%20ref%29))
  (CallFunction|AddtoScore OtherActor 5))

(event EventBeginPlay
  (bind _asmy_game_mode (Utilities|Casting|CastToMyGameMode (Game|GetGameMode)))
  (Variables|Default|SetGameMode _asmy_game_mode))

(fn ConstructionScript
  (bind _interptomovement (Variables|Default|GetInterpToMovement))
  (Variables|/Script/Engine.InterpToMovementComponent|SetControlPoints _interptomovement (Utilities|Array|MakeArray (Utilities|Struct|MakeInterpControlPoint (Variables|Default|GetLocation1) true) (Utilities|Struct|MakeInterpControlPoint (Variables|Default|GetLocation2) true)))
  (Variables|/Script/Engine.InterpToMovementComponent|SetDuration _interptomovement (Variables|Default|Getduration)))

(fn AddtoScore
  (params (Other%20Actor :type Actor%20Object%20Reference) (SumAmount :type Integer))
  (bind _gamemode (Variables|Default|GetGameMode))
  (Utilities|Casting|CastToBP_NewArrow Other%20Actor)
  (Variables|/Game/Gamemode/MyGameMode.MyGameMode_C|SetScore _gamemode (+ (Variables|/Game/Gamemode/MyGameMode.MyGameMode_C|GetScore _gamemode) SumAmount)))