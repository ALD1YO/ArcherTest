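; BP_Bow is a bow weapon that builds a draw charge and holds and launches BP_Arrow actors.
; A timeline drives ChargeAmount, playing on begin, reversing on end and resetting on stop.
; Reload spawns an arrow on the bow mesh socket; OldBowFire detaches it, fires it with ChargeAmount and stops the charge.
; An older charge system remains alongside the new one, which drops the valid-arrow check.
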(event Custom|BeginCharge_Old
  ;[1 1 1] Old Charging System
  (Variables|Default|GetArrow
    (:then
      (bind _chargeamount (Timeline|Timeline_0 Play)
        (:Update
          (Variables|Default|SetChargeAmount _chargeamount))))
    (:else)))

(event Custom|EndCharge_Old
  ;[1 1 1] Old Charging System
  (Variables|Default|GetArrow
    (:then
      (bind _chargeamount (Timeline|Timeline_0 Reverse)
        (:Update
          (Variables|Default|SetChargeAmount _chargeamount))))
    (:else)))

(event Custom|StopCharge_Old
  ;[1 1 1] Old Charging System
  (Utilities|FlowControl|Sequence
    (:then_0
      (bind _chargeamount (Timeline|Timeline_0 Stop)
        (:Update
          (Variables|Default|SetChargeAmount _chargeamount))))
    (:then_1
      (Timeline|Timeline_0 SetNewTime))))

(event Custom|OldBowFire
  (bind _arrow (Variables|Default|GetArrow)
    (:then
      (Transformation|DetachFromActor _arrow "KeepWorld" "KeepWorld" "KeepWorld")
      (Default|Fire (Variables|Default|GetArrow) (Variables|Default|GetChargeAmount))
      (Variables|Default|SetArrow 0)
      (CallFunction|StopCharge))
    (:else)))

(event Custom|Reload
  (bind _returnvalue (Game|SpawnActorfromClass "/Game/Blueprints/BP_Arrow.BP_Arrow_C" (Math|Transform|MakeTransform "0, 0, 0" "0, 0, 0" "1,1,1") "Undefined" 0 "NewEnumerator2" 0))
  (bind _output_get (Variables|Default|SetArrow _returnvalue))
  (Transformation|AttachComponentToComponent _output_get (Variables|Default|GetBowMesh) "arrow_attach_socket" "SnapToTarget" "SnapToTarget" "KeepWorld" true))

(event Custom|BeginCharge
  ;[1 1 1] New Charging System
  (bind _chargeamount (Timeline|ChargeTimeline Play)
    (:Update
      (Variables|Default|SetChargeAmount _chargeamount))))

(event Custom|EndCharge
  ;[1 1 1] New Charging System
  (bind _chargeamount (Timeline|ChargeTimeline Reverse)
    (:Update
      (Variables|Default|SetChargeAmount _chargeamount))))

(event Custom|StopCharge
  ;[1 1 1] New Charging System
  (Utilities|FlowControl|Sequence
    (:then_0
      (bind _chargeamount (Timeline|ChargeTimeline Stop)
        (:Update
          (Variables|Default|SetChargeAmount _chargeamount))))
    (:then_1
      (Timeline|ChargeTimeline SetNewTime))))

(fn ConstructionScript)