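; Arrow projectile whose launch speed scales with the bow's charge and which goes inert when its movement stops.
; The construction script loops over all BP_Bow actors and sets InitialSpeed from ChargeAmount times SpeedMultiplier, so the last bow found wins.
; On projectile stop, it zeroes the rotating movement and disables physics and collision.
; An unwired, deprecated chain once rotated the arrow toward the player's camera raycast endpoint.
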(event OnProjectileStop(ProjectileMovement)
  (params (ImpactResult :type Hit%20Result%20Structure%20%28by%20ref%29))
  (Variables|/Script/Engine.RotatingMovementComponent|SetRotationRate (Variables|Default|GetRotatingMovement) "0, 0, 0")
  (Physics|SetSimulatePhysics (Variables|Default|GetCollision%20Component) false)
  (Collision|SetCollisionEnabled (Variables|Default|GetCollision%20Component) "NoCollision"))

(fn ConstructionScript
  (bind _outactors (Actor|GetAllActorsOfClass "/Game/Blueprints/BP_Bow.BP_Bow_C"))
  (for _array_element _outactors
    (bind _output_get (Variables|Default|SetSpeed (* (Variables|/Game/Blueprints/BP_Bow.BP_Bow_C|GetChargeAmount _array_element) (Variables|Default|GetSpeed%20Multiplier))))
    (Variables|/Script/Engine.ProjectileMovementComponent|SetInitialSpeed (Variables|Default|GetProjectileMovement) _output_get)))