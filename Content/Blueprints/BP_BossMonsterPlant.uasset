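; BP_BossMonsterPlant is a monster-plant boss that creates a health widget on spawn and takes damage from player arrows.
; In static mode without homing, it repeatedly fires fast fireballs toward the player; non-static, it melees the player on capsule contact after a windup.
; Tick always issues AIMoveTo at the player controller while alive, leaving the turn-to-face branch unreachable.
; An arrow hit at zero health plays a death reaction, shows a thanks screen, moves EndGate and destroys the boss.
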(event OnComponentHit(CapsuleComponent)
  (params (HitComponent :type Primitive%20Component%20Object%20Reference) (OtherActor :type Actor%20Object%20Reference) (OtherComp :type Primitive%20Component%20Object%20Reference) (NormalImpulse :type Vector :default "0, 0, 0") (Hit :type Hit%20Result%20Structure%20%28by%20ref%29))
  (bind _mesh (Variables|Character|GetMesh))
  (bind _asbp_new_arrow (Utilities|Casting|CastToBP_NewArrow OtherActor)
    (:then
      (Game|Damage|ApplyDamage self 7.0 0 0)
      (if (<= (Variables|Default|GetcurrentHealth) 0.0)
        (Variables|Default|SetisDead? true)
        (Collision|SetCollisionEnabled (Variables|Collision|GetCapsuleComponent) "NoCollision")
        (Components|Animation|PlayAnimation _mesh "/Game/Assets/PlantMonster/Animations/GotHit.GotHit" false)
        (Components|Timeline|SetPlayRate _mesh 1.5)
        (Development|PrintString "Hit")
        (Utilities|FlowControl|Delay 1.2)
        (Viewport|RemoveAllWidgets)
        (bind _returnvalue (UserInterface|CreateWidget "/Game/UI/Thanks_Widget.Thanks_Widget_C"))
        (UserInterface|Viewport|AddtoViewport _returnvalue 0)
        (Transformation|SetActorLocation (Variables|Default|GetEndGate) (Variables|Default|GetEndGateLocation) false false)
        (Actor|DestroyActor _asbp_new_arrow)
        (Actor|DestroyActor)))
    (:CastFailed
      (if (not (Variables|Default|GetisStatic))
        (if (not (Variables|Default|GetisAttacking?))
          (Utilities|Casting|CastToPlayerCharacter OtherActor)
          (Components|Animation|PlayAnimation (Variables|Character|GetMesh) "/Game/Assets/PlantMonster/Animations/Attack01.Attack01" false)
          (Variables|Default|SetisAttacking? true)
          (Utilities|FlowControl|Delay 0.7)
          (if (not (Variables|Default|GetisDead?))
            (Game|Damage|ApplyDamage (Game|GetPlayerCharacter 0) (Variables|Default|GetattackPower) 0 0)
            (Utilities|FlowControl|Delay 1.2)
            (Variables|Default|SetisAttacking? false)
            (Components|Animation|PlayAnimation (Variables|Character|GetMesh) "/Game/Assets/PlantMonster/Animations/AttackIdle.AttackIdle" true)
            (Development|PrintString "character")))))))

(event Game|Damage|EventAnyDamage
  (params (Damage :type Float%20%28single-precision%29) (DamageType :type Damage%20Type%20Object%20Reference) (InstigatedBy :type Controller%20Object%20Reference) (DamageCauser :type Actor%20Object%20Reference))
  (bind _output_get (Variables|Default|SetcurrentHealth (- (Variables|Default|GetcurrentHealth) Damage)))
  (Development|PrintString (Utilities|String|ToString(Float) _output_get)))

(event EventTick
  (params (DeltaSeconds :type Float%20%28single-precision%29))
  (bind _capsulecomponent (Variables|Collision|GetCapsuleComponent))
  (if (Variables|Default|GetisDead?)
    (Components|Movement|StopMovementImmediately (Variables|Character|GetCharacterMovement))
    (elif true
      (AI|AIMoveTo self "0, 0, 0" (Game|GetPlayerController 0) (Variables|Default|GetAttackDistance) false
        (:then
          (if (<= (- (Math|Vector|Distance(Vector) (Transformation|GetActorLocation) (Transformation|GetActorLocation (Game|GetPlayerCharacter 0))) 1e+02) (Variables|Default|GetAttackDistance))
            _)))
      (else
        (Transformation|SetWorldRotation _capsulecomponent (Math|Rotator|FindLookatRotation (Transformation|GetWorldLocation _capsulecomponent) (Transformation|GetActorLocation (Game|GetPlayerCharacter 0))) false false)))))

(event EventBeginPlay
  (bind _spawnprojectile (Variables|Default|GetSpawnProjectile))
  (bind _maxwalkspeed (Variables|Default|GetmaxWalkSpeed))
  (bind _charactermovement (Variables|Character|GetCharacterMovement))
  (bind _returnvalue (UserInterface|CreateWidget "/Game/UI/BossHealth_Widget.BossHealth_Widget_C"))
  (UserInterface|Viewport|AddtoViewport _returnvalue 0)
  ;[1 1 1] see the monster
  (Utilities|FlowControl|Delay 4.0)
  (if (Variables|Default|GetisStatic)
    (Variables|/Script/Engine.CharacterMovementComponent|SetMaxWalkSpeed _charactermovement _maxwalkspeed)
    (Components|Animation|PlayAnimation (Variables|Character|GetMesh) "/Game/Assets/PlantMonster/Animations/Attack01_NoSound.Attack01_NoSound" false :!label _label)
    (Transformation|SetWorldRotation _spawnprojectile (Math|Rotator|FindLookatRotation (Transformation|GetWorldLocation _spawnprojectile) (Transformation|GetActorLocation (Game|GetPlayerCharacter 0))) false false)
    (if (not (Variables|Default|GetisHomingProjectile?))
      (Utilities|FlowControl|Delay 0.1)
      (Game|SpawnActorfromClass "/Game/Blueprints/BP_FireballFast.BP_FireballFast_C" (Transformation|GetWorldTransform (Variables|Default|GetSpawnProjectile)) "Undefined" 0 0)
      (Utilities|FlowControl|Delay (Variables|Default|GetfireRate))
      (if (not (Variables|Default|GetisDead?))
        (goto _label)))
    (else
      (Variables|/Script/Engine.CharacterMovementComponent|SetMaxWalkSpeed _charactermovement _maxwalkspeed))))

(fn ConstructionScript)